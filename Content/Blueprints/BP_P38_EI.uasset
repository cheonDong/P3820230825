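; BP_P38_EI is a player-flown P-38 plane that constantly moves along its forward vector, driven by Enhanced Input actions.
; Pitch-and-roll input applies frame-time-scaled local rotations, while boost input raises the per-tick movement scale until released.
; On BeginPlay it registers the Right and Left components, likely propellers, with a rotating scene component to spin about X.
; A RotatePropeller function exists but is not called here, and a test action prints its value.
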(event `self.ReceiveBeginPlay`
  (`/Game/Blueprints/BP_RotatingStaticMeshComponent.AddSceneComponent` (`self.BP_RotatingSceneComponent`) (`self.Right`))
  (`/Game/Blueprints/BP_RotatingStaticMeshComponent.AddSceneComponent` (`self.BP_RotatingSceneComponent`) (`self.Left`))
  (set `/Game/Blueprints/BP_RotatingStaticMeshComponent.Axis` (struct :`Roll` 1.0) (`self.BP_RotatingSceneComponent`)))

(event `self.ReceiveTick`
  (params (DeltaSeconds :type "Float (single-precision)"))
  (`self.AddMovementInput` (`self.GetActorForwardVector`) (`self.Boost`)))

(event `EnhancedInput|/Game/Blueprints/Input/IA_Test`
  (params (ActionValue :type Boolean) (ElapsedSeconds :type "Float (double-precision)") (TriggeredSeconds :type "Float (double-precision)") (InputAction :type "InputAction Object Reference" :default "/Game/Blueprints/Input/IA_Test.IA_Test"))
  (:`Triggered`
    (`KismetSystemLibrary.PrintString` (`KismetStringLibrary.Conv_BoolToString` ActionValue))))

(event `EnhancedInput|/Game/Blueprints/Input/IA_PitchAndRoll`
  (params (ActionValue :type "Vector2D Structure") (ElapsedSeconds :type "Float (double-precision)") (TriggeredSeconds :type "Float (double-precision)") (InputAction :type "InputAction Object Reference" :default "/Game/Blueprints/Input/IA_PitchAndRoll.IA_PitchAndRoll"))
  (:`Triggered`
    ;[1 1 1] Roll
    (`self.K2_AddActorLocalRotation` (`KismetMathLibrary.MakeRotator` (* ActionValue_X (`self.RotationSpeed`) (`GameplayStatics.GetWorldDeltaSeconds`))))
    ;[1 1 1] Pitch
    (`self.K2_AddActorLocalRotation` (`KismetMathLibrary.MakeRotator` 0.0 (* ActionValue_Y (`self.RotationSpeed`) (`GameplayStatics.GetWorldDeltaSeconds`))))))

(event `EnhancedInput|/Game/Blueprints/Input/IA_Boost`
  (params (ActionValue :type Boolean) (ElapsedSeconds :type "Float (double-precision)") (TriggeredSeconds :type "Float (double-precision)") (InputAction :type "InputAction Object Reference" :default "/Game/Blueprints/Input/IA_Boost.IA_Boost"))
  (:`Triggered`
    (set `self.Boost` 1.0))
  (:`Canceled`
    (set `self.Boost` 0.5 :!label _label))
  (:`Completed`
    (goto _label)))

(fn `RotatePropeller`
  (params (Where :type "SceneComponent Object Reference"))
  (`SceneComponent.K2_AddLocalRotation` Where (`KismetMathLibrary.MakeRotator` (* (`GameplayStatics.GetWorldDeltaSeconds`) (`self.Speed`))) false false))

(fn `UserConstructionScript`)